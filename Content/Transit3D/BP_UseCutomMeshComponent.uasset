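; Test actor for Transit3D that procedurally builds geometry on a CustomMesh component, starting from a placeholder triangle in construction.
; SB events compute and apply a sine-wave strip.
; The DataTable test, triggered manually or by an editor tick, rebuilds SBTriangles by joining each row's four-corner section (X, Y, time as Z) to the previous one, forming a tube.
; GetFirstRowOfDt can seed that previous section but is never called here.
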(event `self.ReceiveTick`
  (params (DeltaSeconds :type "Float (single-precision)"))
  (`KismetSystemLibrary.PrintString` (`KismetTextLibrary.Conv_TextToString` (`KismetTextLibrary.AsTime_DateTime` (`KismetMathLibrary.Now`)))))

(event `SB_Modifiy`
  (`CustomMeshComponent.SetCustomMeshTriangles` (`self.CustomMesh`) (`|MakeArray` (make `CustomMeshTriangle` (0.0 0.0 0.0) (0.0 50.0 50.0) (0.0 0.0 50.0)))))

(event `SB_Compute`
  (`|ExecutionSequence`
    (:`then_0`
      (set `self.SB_V0a` (0.0 0.0 0.0))
      (set `self.SB_V0b` (`KismetMathLibrary.MakeVector` 0.0 (`self.SB_Depth`))))
    (:`then_1`
      (for _index (range 1 (+ (`self.SB_GranularityFactor`) 1))
        (`|ExecutionSequence`
          (:`then_0`
            (bind _returnvalue (`KismetMathLibrary.Conv_IntToDouble` (`KismetMathLibrary.FTrunc` (* (`KismetMathLibrary.MultiplyByPi` (`KismetMathLibrary.Conv_IntToDouble` _index)) 2.0))))
            (bind _returnvalue_2 (* (/ _returnvalue (`self.SB_GranularityFactor`)) (`self.SB_Length`)))
            (bind _returnvalue_3 (* (`KismetMathLibrary.Sin` (* (/ _returnvalue (`self.SB_GranularityFactor`)) 2.0)) (`self.SB_Height`)))
            (set `self.SB_Temp_V1a` (`KismetMathLibrary.MakeVector` _returnvalue_2 0.0 _returnvalue_3))
            (set `self.SB_Temp_V1b` (`KismetMathLibrary.MakeVector` _returnvalue_2 (`self.SB_Depth`) _returnvalue_3))
            (`KismetArrayLibrary.Array_Add` (`self.SB_Triangles`) (make `CustomMeshTriangle` (`self.SB_V0a`) (`self.SB_V0b`) (`self.SB_Temp_V1a`)))
            (`KismetArrayLibrary.Array_Add` (`self.SB_Triangles`) (make `CustomMeshTriangle` (`self.SB_Temp_V1a`) (`self.SB_V0b`) (`self.SB_Temp_V1b`))))
          (:`then_1`
            (set `self.SB_V0a` (`self.SB_Temp_V1a`))
            (set `self.SB_V0b` (`self.SB_Temp_V1b`))))))))

(event `SB_Set`
  (`CustomMeshComponent.SetCustomMeshTriangles` (`self.CustomMesh`) (`self.SB_Triangles`)))

(event `Do_Test_with_DT_Mesh_036_12512_CSV`
  (`self.Test With DT Mesh 036 15h 12 Csv` null :!label _label))

(event `/Game/Tick_in_editor_based_on_httpsdotdotbsbsdevdotepicgamesdotcomscommunityslearningstutorialssPBnRscreating-an-editor-tick-in-unreal-engine/BPI_Transit3D_EditorTick.Transit 3D Editor Tick`
  ;[1 1 1] Based on https://dev.epicgames.com/community/learning/tutorials/PBnR/creating-an-editor-tick-in-unreal-engine
  (`KismetSystemLibrary.PrintString` "ddssaa")
  (goto _label))

(fn `GetAndAddOtherRowsOfDt`
  (bind _verticespreviousdtrow (`self.VerticesPreviousDtRow`))
  (bind _mytestdatatable (`self.MyTestDataTable`))
  (bind _output (`|GetArrayItem` _verticespreviousdtrow 3))
  (bind _output_2 (`|GetArrayItem` _verticespreviousdtrow))
  (bind _output_3 (`|GetArrayItem` _verticespreviousdtrow 2))
  (bind _output_4 (`|GetArrayItem` _verticespreviousdtrow 1))
  (bind _outrownames (`DataTableFunctionLibrary.GetDataTableRowNames` _mytestdatatable))
  (for _array_element _outrownames
    (`KismetSystemLibrary.PrintString` (`KismetStringLibrary.Conv_NameToString` _array_element))
    (bind _returnvalue (`|GetDataTableRow` _mytestdatatable _array_element)
      (:`then`
        (`|ExecutionSequence`
          (:`then_1`
            (bind (_topfastleftx _topfastlefty _topfastlefttimez _topfastrightx _topfastrighty _topfastrighttimez _bottomslowrightx _bottomslowrighty _bottomslowrighttimez _bottomslowleftx _bottomslowlefty _bottomslowlefttimez) (break `/Game/MeshTests/S_Transit3DFourVerticesOfATime` _returnvalue))
            (bind _returnvalue_2 (`KismetMathLibrary.MakeVector_NetQuantize` _topfastleftx _topfastlefty _topfastlefttimez))
            (bind _returnvalue_3 (`KismetMathLibrary.MakeVector_NetQuantize` _topfastrightx _topfastrighty _topfastrighttimez))
            (bind _returnvalue_4 (`KismetMathLibrary.MakeVector_NetQuantize` _bottomslowrightx _bottomslowrighty _bottomslowrighttimez))
            (bind _returnvalue_5 (`KismetMathLibrary.MakeVector_NetQuantize` _bottomslowleftx _bottomslowlefty _bottomslowlefttimez))
            (`KismetArrayLibrary.Array_Append` (`self.SB_Triangles`) (`|MakeArray` (make `CustomMeshTriangle` _output_2 _output_4 _returnvalue_2) (make `CustomMeshTriangle` _returnvalue_2 _output_4 _returnvalue_3) (make `CustomMeshTriangle` _output_4 _output_3 _returnvalue_3) (make `CustomMeshTriangle` _returnvalue_3 _output_3 _returnvalue_4) (make `CustomMeshTriangle` _output_3 _output _returnvalue_4) (make `CustomMeshTriangle` _returnvalue_4 _output _returnvalue_5) (make `CustomMeshTriangle` _output _output_2 _returnvalue_5) (make `CustomMeshTriangle` _returnvalue_5 _output_2 _returnvalue_2)))
            (set `self.VerticesPreviousDtRow` (`|MakeArray` _returnvalue_2 _returnvalue_3 _returnvalue_4 _returnvalue_5 :!type "Vector Structure"))))))))

(fn `GetFirstRowOfDt`
  (bind _outrownames (`DataTableFunctionLibrary.GetDataTableRowNames` (`self.MyTestDataTable`)))
  (bind _returnvalue (`|GetDataTableRow` (`self.MyTestDataTable`) (`|GetArrayItem` _outrownames))
    (:`then`
      (bind _output_get (set `self.PreivousDtRow` _returnvalue))
      (bind (_topfastleftx _topfastlefty _topfastlefttimez _topfastrightx _topfastrighty _topfastrighttimez _bottomslowrightx _bottomslowrighty _bottomslowrighttimez _bottomslowleftx _bottomslowlefty _bottomslowlefttimez) (break `/Game/MeshTests/S_Transit3DFourVerticesOfATime` _output_get))
      (set `self.VerticesPreviousDtRow` (`|MakeArray` (`KismetMathLibrary.MakeVector_NetQuantize` _topfastleftx _topfastlefty _topfastlefttimez) (`KismetMathLibrary.MakeVector_NetQuantize` _topfastrightx _topfastrighty _topfastrighttimez) (`KismetMathLibrary.MakeVector_NetQuantize` _bottomslowrightx _bottomslowrighty _bottomslowrighttimez) (`KismetMathLibrary.MakeVector_NetQuantize` _bottomslowleftx _bottomslowlefty _bottomslowlefttimez) :!type "Vector Structure")))))

(fn `Test With DT Mesh 036 15h 12 Csv`
  (params (MyDynamicMesh :type "DynamicMesh Object Reference"))
  (bind _returnvalue (`DynamicMesh.GetTriangleCount` (`local.MyDynamicMesh`)))
  (set `self.MyDynamicMesh` MyDynamicMesh)
  (`|ExecutionSequence`
    (:`then_0`
      (`KismetArrayLibrary.Array_Clear` (`self.SB_Triangles`)))
    (:`then_1`
      (`KismetSystemLibrary.PrintString` (`KismetStringLibrary.Concat_StrStr` "There were " (`KismetStringLibrary.Conv_IntToString` _returnvalue) "Triangles"))
      ;[1 1 1] Delete previous triangles
      (for _index (range _returnvalue 1)
        (`GeometryScriptLibrary_MeshBasicEditFunctions.DeleteTriangleFromMesh` (`local.MyDynamicMesh`) _index)))
    (:`then_3`
      (`self.GetAndAddOtherRowsOfDt`))
    (:`then_4`
      (`CustomMeshComponent.SetCustomMeshTriangles` (`self.CustomMesh`) (`self.SB_Triangles`)))))

(fn `UserConstructionScript`
  (`|ExecutionSequence`
    (:`then_0`
      (`CustomMeshComponent.SetCustomMeshTriangles` (`self.CustomMesh`) (`|MakeArray` (make `CustomMeshTriangle` (0.0 0.0 0.0) (0.0 100.0 100.0) (0.0 0.0 100.0)))))
    (:`then_1`
      (`AddComponent|NODE_AddChildActorComponent-0`))))